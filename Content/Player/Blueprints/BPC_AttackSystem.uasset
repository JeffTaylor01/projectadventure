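; Player attack component that runs a three-hit montage combo on BP_Player's mesh from IA_Attack input, gated by CanAttack.
; SwordAttack starts the montage selected by AttackIndex, or buffers presses in SaveAttack while attacking.
; Each DoOnce-guarded attack waits briefly, plays its montage and advances the index.
; ComboContinue, not called within this graph, consumes the buffer to chain the next hit, otherwise StopCombo resets the state.
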(event Custom|Combo%20Continue
  ;[0.05098 0.05098 0.05098] Continue Combo
  (if (Variables|Default|GetsaveAttack)
    (Variables|Default|SetsaveAttack false)
    (switch int (Variables|Default|GetattackIndex)
      (:0
        (CallFunction|Attack1))
      (:1
        (CallFunction|Attack2))
      (:2
        (CallFunction|Attack3)))
    (else
      (CallFunction|StopCombo))))

(event Custom|Stop%20Combo
  ;[0.05098 0.05098 0.05098] Stop Combo
  (Variables|Default|SetisAttacking false)
  (Variables|Default|SetattackIndex 0))

(event Custom|Sword%20Attack
  ;[0.05098 0.05098 0.05098] Sword Attack
  (if (Variables|Default|GetisAttacking)
    (Variables|Default|SetsaveAttack true)
    (else
      (Variables|Default|SetisAttacking true)
      (switch int (Variables|Default|GetattackIndex)
        (:0
          (CallFunction|Attack1))
        (:1
          (CallFunction|Attack2))
        (:2
          (CallFunction|Attack3))))))

(event Custom|Attack%201
  ;[0.05098 0.05098 0.05098] Attack 1
  (Utilities|FlowControl|DoOnce false :!label _label
    (:Completed
      (Utilities|FlowControl|Delay 0.1)
      (Animation|Montage|PlayMontage (Variables|Default|GetCharacter%20Mesh) "/Game/Player/Animations/SwordAttacks/SwordOutwardSlash_Montage.SwordOutwardSlash_Montage"
        (:then
          (Variables|Default|SetattackIndex 1)
          (goto _label Reset))))))

(event Custom|Attack%202
  ;[0.05098 0.05098 0.05098] Attack 2
  (Utilities|FlowControl|DoOnce false :!label _label
    (:Completed
      (Utilities|FlowControl|Delay 0.1)
      (Animation|Montage|PlayMontage (Variables|Default|GetCharacter%20Mesh) "/Game/Player/Animations/SwordAttacks/Attack2_UE_Montage.Attack2_UE_Montage"
        (:then
          (Variables|Default|SetattackIndex 2)
          (goto _label Reset))))))

(event Custom|Attack%203
  ;[0.05098 0.05098 0.05098] Attack 3
  (Utilities|FlowControl|DoOnce false :!label _label
    (:Completed
      (Utilities|FlowControl|Delay 0.1)
      (Animation|Montage|PlayMontage (Variables|Default|GetCharacter%20Mesh) "/Game/Player/Animations/SwordAttacks/Attack3_UE_Montage.Attack3_UE_Montage"
        (:then
          (Variables|Default|SetattackIndex 3)
          (goto _label Reset))))))

(event Input|EnhancedActionEvents|EnhancedInputActionIA_Attack
  (params (ActionValue :type Boolean) (ElapsedSeconds :type Float%20%28double-precision%29) (TriggeredSeconds :type Float%20%28double-precision%29) (InputAction :type Input%20Action%20Object%20Reference :default "/Game/Player/Input/Actions/IA_Attack.IA_Attack"))
  ;[0.05098 0.05098 0.05098] Attack Input
  (:Started
    (if (Variables|Default|GetcanAttack)
      (CallFunction|SwordAttack))))

(event EventBeginPlay
  (bind _asbp_player (Utilities|Casting|CastToBP_Player (Components|GetOwner)))
  (Variables|Default|SetCharacter%20Mesh (Variables|/Script/Engine.Character|GetMesh _asbp_player)))